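; TargetBHard is a target Blueprint that takes two hits to destroy.
; The first Hit event sets the BeenHit flag and swaps the static mesh to a red material.
; The next hit sends a raw score message to the player pawn, plays the B_Hit sound at the target's location and destroys the actor.
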(event `/Game/Blueprints/Interfaces/BPI_Enmy.Hit`
  (if (`self.BeenHit`)
    (message `/Game/Blueprints/Interfaces/BPI_Player.AddRawScore` (`GameplayStatics.GetPlayerPawn` 0) 1)
    (`GameplayStatics.SpawnSoundAtLocation` "/Game/Sounds/B_Hit.B_Hit" (`SceneComponent.K2_GetComponentLocation` (`self.Root`)))
    (`self.K2_DestroyActor`)
    (else
      (set `self.BeenHit` true)
      (`PrimitiveComponent.SetMaterial` (`self.StaticMesh`) 0 "/Game/Import/Textures/target_texture_red_Mat.target_texture_red_Mat"))))

(fn `UserConstructionScript`)