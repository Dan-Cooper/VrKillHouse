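; Spawner actor that places a single target at its root transform when play begins.
; The IsHard flag selects TargetBHard; otherwise IsGood chooses between TargetG and TargetB, with Speed passed as the target's StartSpeed.
; A separate InSpawn event calls SpawnEnemy, which always spawns a TargetB without passing Speed.
; All spawns ignore collisions.
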(event `self.ReceiveBeginPlay`
  (bind _speed (`self.Speed`))
  (bind _returnvalue (`SceneComponent.K2_GetComponentToWorld` (`self.Root`)))
  (if (`self.IsHard`)
    (`|SpawnActorFromClass` "/Game/Blueprints/Targets/TargetBHard.TargetBHard_C" _returnvalue "AlwaysSpawn" "OverrideRootScale" null _speed null)
    (elif (`self.IsGood`)
      (`|SpawnActorFromClass` "/Game/Blueprints/Targets/TargetG.TargetG_C" _returnvalue "AlwaysSpawn" "OverrideRootScale" null _speed null)
      (else
        (`|SpawnActorFromClass` "/Game/Blueprints/Targets/TargetB.TargetB_C" _returnvalue "AlwaysSpawn" "OverrideRootScale" null _speed null)))))

(event `/Game/Blueprints/Interfaces/BPI_Spawner.In_Spawn`
  (`self.SpawnEnemy`))

(fn `SpawnEnemy`
  (`|SpawnActorFromClass` "/Game/Blueprints/Targets/TargetB.TargetB_C" (`SceneComponent.K2_GetComponentToWorld` (`self.Root`)) "AlwaysSpawn" "OverrideRootScale" null 0.0 null))

(fn `UserConstructionScript`)