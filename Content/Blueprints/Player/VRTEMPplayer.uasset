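; VR player Blueprint that handles shooting, teleport movement and the player's raw score.
; The right trigger line-traces from the gun, spawns impact effects and messages hit enemies or in-game menus through interfaces.
; Each tick a trace marks near-flat surfaces with a debug cylinder; left thumbstick press moves the player there, offset by the left controller's relative XY.
; Score changes are pushed to the first score-interface actor found at BeginPlay.
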(event `self.ReceiveBeginPlay`
  ;[1 1 1] Controles Score
  (bind _outactors (`GameplayStatics.GetAllActorsWithInterface` "/Game/Blueprints/UI/BPI_InGameScore.BPI_InGameScore_C"))
  (set `self.ScoreBP` (`|GetArrayItem` _outactors)))

(event `/Game/Blueprints/Interfaces/BPI_Player.AddRawScore`
  (params (Val :type Integer))
  ;[1 1 1] Controles Score
  (bind _output_get (set `self.RawScore` (+ Val (`self.RawScore`))))
  (message `/Game/Blueprints/UI/BPI_InGameScore.UpdateDisplayS` (`self.ScoreBP`) _output_get))

(event `/Game/Blueprints/Interfaces/BPI_Player.Reset`
  ;[1 1 1] Controles Score
  (set `self.RawScore` 0))

(event `Key|MotionController_Right_Trigger`
  (params (Key :type "Key Structure"))
  (bind _gunend (`self.GunEnd`))
  (bind _returnvalue (`SceneComponent.K2_GetComponentLocation` _gunend))
  ;[1 1 1] FireControle And Hit Detection
  (:`Pressed`
    (`GameplayStatics.SpawnSoundAttached` "/Game/Sounds/Future_Weapons_2_-_Source_-_Laser_Source_3.Future_Weapons_2_-_Source_-_Laser_Source_3" (`self.GunEnd`) "None" (0.0 0.0 0.0) (struct) "KeepRelativeOffset" false 0.6 1.0 1.2)
    (bind (_outhit _returnvalue_2) (`KismetSystemLibrary.LineTraceSingle` :`Start` _returnvalue :`End` (+ _returnvalue (* (`KismetMathLibrary.GetForwardVector` (`SceneComponent.K2_GetComponentRotation` _gunend)) 1500.0)) :`TraceChannel` "TraceTypeQuery1" :`DrawDebugType` "Persistent"))
    (if _returnvalue_2
      (bind (_bblockinghit _binitialoverlap _time _location _impactpoint _normal _impactnormal _physmat _hitactor _hitcomponent) (`GameplayStatics.BreakHitResult` _outhit))
      (set `self.HitActor` _hitactor)
      (`GameplayStatics.SpawnEmitterAtLocation` "/Game/Particals/Impact.Impact" _impactpoint (`KismetMathLibrary.MakeRotFromZ` _impactnormal))
      (if (`KismetSystemLibrary.DoesImplementInterface` (`self.HitActor`) "/Game/Blueprints/Interfaces/BPI_Enmy.BPI_Enmy_C")
        (message `/Game/Blueprints/Interfaces/BPI_Enmy.Hit` (`self.HitActor`))
        (elif (`KismetSystemLibrary.DoesImplementInterface` (`self.HitActor`) "/Game/Blueprints/UI/BPI_InGameMenue.BPI_InGameMenue_C")
          (message `/Game/Blueprints/UI/BPI_InGameMenue.InteractWithMenue` (`self.HitActor`) _hitcomponent))))))

(event `self.ReceiveTick`
  (params (DeltaSeconds :type "Float (single-precision)"))
  (bind _teliportend (`self.Teliportend`))
  ;[1 1 1] Teliport
  (`self.TraceGetTeliportLocation` (`SceneComponent.K2_GetComponentLocation` _teliportend) (`SceneComponent.GetForwardVector` _teliportend)))

(event `Key|MotionController_Left_Thumbstick`
  (params (Key :type "Key Structure"))
  ;[1 1 1] Teliport
  (:`Pressed`
    (if (`self.CanTeliport`)
      (`self.TeliportToLoc` (`self.TeliLoc`)))))

(fn `TeliportToLoc`
  (params (Loc :type "Vector Structure"))
  (bind (_relativelocation_x _relativelocation_y) (`KismetMathLibrary.BreakVector` (`SceneComponent.RelativeLocation` (`self.ViveControlerL`))))
  (`self.K2_SetActorLocation` (+ Loc (`KismetMathLibrary.MakeVector` _relativelocation_x _relativelocation_y))))

(fn `TraceGetTeliportLocation`
  (params (Position :type "Vector Structure") (Forward :type "Vector Structure"))
  (locals (NewLocalVar_0 :type "Array of HitResult Structure") (NewLocalVar_1 :type "Array of HitResult Structure"))
  (bind _outhit (`KismetSystemLibrary.LineTraceSingle` :`Start` Position :`End` (+ Position (* (`KismetMathLibrary.GetForwardVector` (`SceneComponent.K2_GetComponentRotation` (`self.Teliportend`))) 1500.0)) :`TraceChannel` "TraceTypeQuery1" :`DrawDebugType` "ForOneFrame"))
  (bind (_bblockinghit _binitialoverlap _time _location _impactpoint _normal) (`GameplayStatics.BreakHitResult` _outhit))
  (bind _output_get (set `self.CanTeliport` (> (`KismetMathLibrary.Dot_VectorVector` _normal (0.0 0.0 1.0)) 0.75)))
  (if _output_get
    (bind _output_get_2 (set `self.TeliLoc` _impactpoint))
    (`KismetSystemLibrary.DrawDebugCylinder` _output_get_2 (+ _output_get_2 (* _normal 20.0)) 100.0 25 (struct :`R` 0.020612 :`G` 1.0 :`B` 0.980104 :`A` 1.0))))

(fn `UserConstructionScript`)